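; BP_Events runs RoboValley's timed match hazards and twists: spikes, ground break with temporary platforms, player shrink or grow, and ball growth.
; Tick polls counter values and ground state, while IsEventPlayed and DoOnce gates limit overlapping or repeated events.
; Delay chains handle HUD warnings, material flashes and reverting changes.
; A Box overlap increments the right score and respawns the RoboChar; SpeedUp is never called.
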(event `self.ReceiveBeginPlay`
  ;[1 1 1] Event Begin Play
  (bind _asmain_hud (cast `/Game/RoboValley/Blueprints/UI/MainHud` (`PlayerController.GetHUD` (`GameplayStatics.GetPlayerController` 0))))
  (set `self.MainHud REF` _asmain_hud)
  (bind _asrobo_valley_game_mode (cast `/Game/RoboValley/Game/RoboValleyGameMode` (`GameplayStatics.GetGameMode`)))
  (set `self.Gamemode REF` _asrobo_valley_game_mode))

(event `self.ReceiveTick`
  (params (DeltaSeconds :type "Float (single-precision)"))
  ;[1 1 1] Event Tick
  (`self.Spikes`)
  (`self.BreakGround`)
  (`self.Grow`)
  (`self.Shrink`)
  (`self.GrowBall`))

(event `GrowBall`
  (bind _counter_ref (`self.Counter REF`))
  (bind _sphere (`/Game/RoboValley/Blueprints/BP_Ball.Sphere` (`self.Ball REF`)))
  ;[1 1 1] Grow Up the Ball
  (if (not (`self.IsEventPlayed?`))
    (if (or (== (`/Game/RoboValley/Blueprints/BP_CounterVolleyball_SP.Counter Left` _counter_ref) 5) (== (`/Game/RoboValley/Blueprints/BP_CounterVolleyball_SP.Counter Right` _counter_ref) 5))
      (`/Engine/EditorBlueprintResources/StandardMacros.DoOnce` false
        (:`Completed`
          (set `self.IsEventPlayed?` true)
          (`self.SetWarningScreenVisible`)
          (`self.SetWarningScreenHidden`)
          (`KismetSystemLibrary.Delay` 3.0)
          (`SceneComponent.SetRelativeScale3D` _sphere (2.0 2.0 2.0))
          (`KismetSystemLibrary.Delay` 8.0)
          (`self.SetWarningScreenVisible`)
          (`self.SetWarningScreenHidden`)
          (`KismetSystemLibrary.Delay` 3.0)
          (`SceneComponent.SetRelativeScale3D` _sphere (1.0 1.0 1.0))
          (set `self.IsEventPlayed?` false))))))

(event `BreakGround`
  ;[1 1 1] Break Ground
  (if (not (`self.IsEventPlayed?`))
    (`/Game/RoboValley/Blueprints/Platform/BP_Ground.Ground Disapear` (`self.Ground`))
    (if (`/Game/RoboValley/Blueprints/Platform/BP_Ground.IsGroundDisapear?` (`self.Ground`))
      (`/Engine/EditorBlueprintResources/StandardMacros.DoOnce` false :!label _label
        (:`Completed`
          (set `self.IsEventPlayed?` true)
          (set `self.IsPlatformSpawned?` true)
          (bind _returnvalue (`|SpawnActorFromClass` "/Game/RoboValley/Blueprints/Platform/BP_MovingPlatform2D.BP_MovingPlatform2D_C" (`self.Spawn Transform_1`) "Undefined" "OverrideRootScale" null null))
          (bind _returnvalue_2 (`|SpawnActorFromClass` "/Game/RoboValley/Blueprints/Platform/BP_BreakingPlatform.BP_BreakingPlatform_C" (`self.Spawn Transform`) "Undefined" "OverrideRootScale" null null))
          (bind _returnvalue_3 (`|SpawnActorFromClass` "/Game/RoboValley/Blueprints/Platform/BP_MovingPlatform2D.BP_MovingPlatform2D_C" (`self.Spawn Transform_0`) "Undefined" "OverrideRootScale" null null))
          (`SceneComponent.K2_SetWorldLocation` (`/Game/RoboValley/Blueprints/Platform/BP_MovingPlatform2D.Endpoint` _returnvalue_3) (1200.0 800.0 900.0) false false)
          (`KismetSystemLibrary.Delay` 24.0)
          (set `self.IsPlatformSpawned?` false)
          (set `self.IsEventPlayed?` false)
          (`self.K2_DestroyActor` _returnvalue)
          (`self.K2_DestroyActor` _returnvalue_2)
          (`self.K2_DestroyActor` _returnvalue_3)))
      (elif (not (`self.IsPlatformSpawned?`))
        (goto _label :!via `Reset`)))))

(event `SpeedUp`
  (bind _player_ref (`self.Player REF`))
  (bind _ai_ref (`self.AI REF`))
  (bind _player_ref_2 (`self.Player REF`))
  (bind _ai_ref_2 (`self.AI REF`))
  ;[1 1 1] Speed Up the Ball
  (if (not (`self.IsEventPlayed?`))
    (set `self.IsEventPlayed?` true)
    (set `/Game/RoboValley/Blueprints/Character/BP_RoboChar.MinY` -1800.0 _player_ref_2)
    (set `/Game/RoboValley/Blueprints/Character/BP_RoboChar.MaxY` -2000.0 _player_ref_2)
    (set `/Game/RoboValley/Blueprints/Character/BP_RoboAI.MinY` 1800.0 _ai_ref_2)
    (set `/Game/RoboValley/Blueprints/Character/BP_RoboAI.MaxY` 2000.0 _ai_ref_2)
    (`KismetSystemLibrary.Delay` 15.0)
    (set `/Game/RoboValley/Blueprints/Character/BP_RoboChar.MinY` -800.0 _player_ref)
    (set `/Game/RoboValley/Blueprints/Character/BP_RoboChar.MaxY` -1200.0 _player_ref)
    (set `/Game/RoboValley/Blueprints/Character/BP_RoboAI.MinY` 800.0 _ai_ref)
    (set `/Game/RoboValley/Blueprints/Character/BP_RoboAI.MaxY` 1200.0 _ai_ref)
    (set `self.IsEventPlayed?` false)))

(event `self.Box.OnComponentBeginOverlap`
  (params (OverlappedComponent :type "PrimitiveComponent Object Reference") (OtherActor :type "Actor Object Reference") (OtherComp :type "PrimitiveComponent Object Reference") (OtherBodyIndex :type Integer) (bFromSweep :type Boolean) (SweepResult :type "HitResult Structure (by ref)"))
  ;[1 1 1] Spawn
  (bind _asbp_robo_char (cast `/Game/RoboValley/Blueprints/Character/BP_RoboChar` OtherActor))
  (`/Engine/EditorBlueprintResources/StandardMacros.IncrementInt` (`/Game/RoboValley/Blueprints/UI/WBS_PointCounter.ScoreR` (`/Game/RoboValley/Blueprints/UI/MainHud.WBS PointCounter REF` (`self.MainHud REF`)))
    (:`  `
      (`self.K2_SetActorLocation` _asbp_robo_char (`SceneComponent.K2_GetComponentLocation` (`Actor.RootComponent` (`/Game/RoboValley/Blueprints/Character/BP_RoboChar.PlayerStart` _asbp_robo_char))) false true))))

(event `Shrink`
  (bind _player_ref (`self.Player REF`))
  (bind _counter_ref (`self.Counter REF`))
  (bind _mesh (`Character.Mesh` _player_ref))
  ;[1 1 1] Shrink the player
  (if (not (`self.IsEventPlayed?`))
    (if (or (== (`/Game/RoboValley/Blueprints/BP_CounterVolleyball_SP.Counter Left` _counter_ref) 6) (== (`/Game/RoboValley/Blueprints/BP_CounterVolleyball_SP.Counter Right` _counter_ref) 6))
      (`/Engine/EditorBlueprintResources/StandardMacros.DoOnce` false :!label _label_2
        (:`Completed`
          (set `self.IsEventPlayed?` true)
          (`self.SetWarningScreenVisible`)
          (`self.SetWarningScreenHidden`)
          (`KismetSystemLibrary.Delay` 3.0)
          (set `self.IsShrinked?` true)
          (`PrimitiveComponent.SetMaterial` _mesh 0 "/Game/RoboValley/Material/Red.Red")
          (`KismetSystemLibrary.Delay` 0.3)
          (`PrimitiveComponent.SetMaterial` _mesh 0 null)
          (`KismetSystemLibrary.Delay` 0.3)
          (`PrimitiveComponent.SetMaterial` _mesh 0 "/Game/RoboValley/Material/Red.Red")
          (`KismetSystemLibrary.Delay` 0.2)
          (`PrimitiveComponent.SetMaterial` _mesh 0 null)
          (`KismetSystemLibrary.Delay` 0.2)
          (`PrimitiveComponent.SetMaterial` _mesh 0 "/Game/RoboValley/Material/Red.Red")
          (`KismetSystemLibrary.Delay` 0.2)
          (`PrimitiveComponent.SetMaterial` _mesh 0 null)
          (`KismetSystemLibrary.Delay` 0.2)
          (`PrimitiveComponent.SetMaterial` _mesh 0 "/Game/RoboValley/Material/Red.Red")
          (`KismetSystemLibrary.Delay` 0.2)
          (`PrimitiveComponent.SetMaterial` _mesh 0 null)
          (`self.SetActorScale3D` _player_ref (0.3 0.3 0.3))
          (`KismetSystemLibrary.Delay` 10.0)
          (`self.SetWarningScreenVisible`)
          (`self.SetWarningScreenHidden`)
          (`KismetSystemLibrary.Delay` 3.0)
          (`PrimitiveComponent.SetMaterial` _mesh 0 "/Game/RoboValley/Material/Green.Green")
          (`KismetSystemLibrary.Delay` 0.3)
          (`PrimitiveComponent.SetMaterial` _mesh 0 null)
          (`KismetSystemLibrary.Delay` 0.3)
          (`PrimitiveComponent.SetMaterial` _mesh 0 "/Game/RoboValley/Material/Green.Green")
          (`KismetSystemLibrary.Delay` 0.2)
          (`PrimitiveComponent.SetMaterial` _mesh 0 null)
          (`KismetSystemLibrary.Delay` 0.2)
          (`PrimitiveComponent.SetMaterial` _mesh 0 "/Game/RoboValley/Material/Green.Green")
          (`KismetSystemLibrary.Delay` 0.2)
          (`PrimitiveComponent.SetMaterial` _mesh 0 null)
          (`KismetSystemLibrary.Delay` 0.2)
          (`PrimitiveComponent.SetMaterial` _mesh 0 "/Game/RoboValley/Material/Green.Green")
          (`KismetSystemLibrary.Delay` 0.2)
          (set `self.IsShrinked?` false)
          (set `self.IsEventPlayed?` false)
          (`PrimitiveComponent.SetMaterial` _mesh 0 null)
          (`self.SetActorScale3D` (`self.Player REF`) (1.0 1.0 1.0))))
      (elif (not (`self.IsShrinked?`))
        (goto _label_2 :!via `Reset`)))))

(event `Grow`
  (bind _counter_ref (`self.Counter REF`))
  (bind _player_ref (`self.Player REF`))
  (bind _mesh (`Character.Mesh` _player_ref))
  (bind _mesh_2 (`Character.Mesh` _player_ref))
  ;[1 1 1] Event Grow Up Player
  (if (not (`self.IsEventPlayed?`))
    (if (or (== (`/Game/RoboValley/Blueprints/BP_CounterVolleyball_SP.Counter Left` _counter_ref) 7) (== (`/Game/RoboValley/Blueprints/BP_CounterVolleyball_SP.Counter Right` _counter_ref) 7))
      (`/Engine/EditorBlueprintResources/StandardMacros.DoOnce` false :!label _label_3
        (:`Completed`
          (set `self.IsEventPlayed?` true)
          (`self.SetWarningScreenVisible`)
          (`self.SetWarningScreenHidden`)
          (`KismetSystemLibrary.Delay` 3.0)
          (set `self.IsGrowed` true)
          (`PrimitiveComponent.SetMaterial` _mesh 0 "/Game/RoboValley/Material/Green.Green")
          (`KismetSystemLibrary.Delay` 0.3)
          (`PrimitiveComponent.SetMaterial` _mesh 0 null)
          (`KismetSystemLibrary.Delay` 0.3)
          (`PrimitiveComponent.SetMaterial` _mesh 0 "/Game/RoboValley/Material/Green.Green")
          (`KismetSystemLibrary.Delay` 0.2)
          (`PrimitiveComponent.SetMaterial` _mesh 0 null)
          (`KismetSystemLibrary.Delay` 0.2)
          (`PrimitiveComponent.SetMaterial` _mesh 0 "/Game/RoboValley/Material/Green.Green")
          (`KismetSystemLibrary.Delay` 0.2)
          (`PrimitiveComponent.SetMaterial` _mesh 0 null)
          (`KismetSystemLibrary.Delay` 0.2)
          (`PrimitiveComponent.SetMaterial` _mesh 0 "/Game/RoboValley/Material/Green.Green")
          (`KismetSystemLibrary.Delay` 0.2)
          (`PrimitiveComponent.SetMaterial` _mesh 0 null)
          (`self.SetActorScale3D` _player_ref (2.5 2.5 2.5))
          (`KismetSystemLibrary.Delay` 10.0)
          (`self.SetWarningScreenVisible`)
          (`self.SetWarningScreenHidden`)
          (`KismetSystemLibrary.Delay` 3.0)
          (`PrimitiveComponent.SetMaterial` _mesh_2 0 "/Game/RoboValley/Material/Red.Red")
          (`KismetSystemLibrary.Delay` 0.3)
          (`PrimitiveComponent.SetMaterial` _mesh_2 0 null)
          (`KismetSystemLibrary.Delay` 0.3)
          (`PrimitiveComponent.SetMaterial` _mesh_2 0 "/Game/RoboValley/Material/Red.Red")
          (`KismetSystemLibrary.Delay` 0.2)
          (`PrimitiveComponent.SetMaterial` _mesh_2 0 null)
          (`KismetSystemLibrary.Delay` 0.2)
          (`PrimitiveComponent.SetMaterial` _mesh_2 0 "/Game/RoboValley/Material/Red.Red")
          (`KismetSystemLibrary.Delay` 0.2)
          (`PrimitiveComponent.SetMaterial` _mesh_2 0 null)
          (`KismetSystemLibrary.Delay` 0.2)
          (`PrimitiveComponent.SetMaterial` _mesh_2 0 "/Game/RoboValley/Material/Red.Red")
          (`KismetSystemLibrary.Delay` 0.2)
          (`PrimitiveComponent.SetMaterial` _mesh_2 0 null)
          (set `self.IsGrowed` false)
          (set `self.IsEventPlayed?` false)
          (`self.SetActorScale3D` _player_ref (1.0 1.0 1.0))))
      (elif (not (`self.IsGrowed`))
        (goto _label_3 :!via `Reset`)))))

(event `SetWarningScreenHidden`
  (bind _wbs_warning (`/Game/RoboValley/Blueprints/UI/MainHud.WBS Warning` (`self.MainHud REF`)))
  ;[1 1 1] Warning Screen Function
  (`KismetSystemLibrary.Delay` 6.0)
  (`/Game/RoboValley/Blueprints/UI/WBS_Warning.Set Hidden` _wbs_warning)
  (`UserWidget.StopAnimation` _wbs_warning (`/Game/RoboValley/Blueprints/UI/WBS_Warning.NewAnimation` _wbs_warning)))

(event `SetWarningScreenVisible`
  (bind _wbs_warning (`/Game/RoboValley/Blueprints/UI/MainHud.WBS Warning` (`self.MainHud REF`)))
  ;[1 1 1] Warning Screen Function
  (`/Game/RoboValley/Blueprints/UI/WBS_Warning.Set Visible` _wbs_warning)
  (`UserWidget.PlayAnimation` _wbs_warning (`/Game/RoboValley/Blueprints/UI/WBS_Warning.NewAnimation` _wbs_warning) 0.0 1 "Forward" 1.0 false))

(event `Spikes`
  (bind _counter_ref (`self.Counter REF`))
  (bind _counter_left (`/Game/RoboValley/Blueprints/BP_CounterVolleyball_SP.Counter Left` _counter_ref))
  (bind _counter_right (`/Game/RoboValley/Blueprints/BP_CounterVolleyball_SP.Counter Right` _counter_ref))
  (bind _cube (`/Game/RoboValley/Blueprints/Platform/BP_Ground.Cube` (`self.Ground`)))
  ;[1 1 1] Spikes
  (if (not (`self.IsEventPlayed?`))
    (if (or (== _counter_left 2) (== _counter_right 2) (== _counter_left 8) (== _counter_right 8))
      (`/Engine/EditorBlueprintResources/StandardMacros.DoOnce` false :!label _label_4
        (:`Completed`
          (set `self.IsEventPlayed?` true)
          (`self.SetWarningScreenVisible`)
          (`self.SetWarningScreenHidden`)
          (`PrimitiveComponent.SetMaterial` _cube 0 "/Game/RoboValley/Material/Red.Red")
          (`KismetSystemLibrary.Delay` 0.4)
          (`PrimitiveComponent.SetMaterial` _cube 0 "/Game/RoboValley/Material/NewMaterial.NewMaterial")
          (`KismetSystemLibrary.Delay` 0.4)
          (`PrimitiveComponent.SetMaterial` _cube 0 "/Game/RoboValley/Material/Red.Red")
          (`KismetSystemLibrary.Delay` 0.4)
          (`PrimitiveComponent.SetMaterial` _cube 0 "/Game/RoboValley/Material/NewMaterial.NewMaterial")
          (`KismetSystemLibrary.Delay` 0.4)
          (`PrimitiveComponent.SetMaterial` _cube 0 "/Game/RoboValley/Material/Red.Red")
          (`KismetSystemLibrary.Delay` 0.4)
          (`PrimitiveComponent.SetMaterial` _cube 0 "/Game/RoboValley/Material/NewMaterial.NewMaterial")
          (`KismetSystemLibrary.Delay` 0.4)
          (`PrimitiveComponent.SetMaterial` _cube 0 "/Game/RoboValley/Material/Red.Red")
          (`KismetSystemLibrary.Delay` 0.4)
          (`PrimitiveComponent.SetMaterial` _cube 0 "/Game/RoboValley/Material/NewMaterial.NewMaterial")
          (set `self.IsSpikeSpawned?` true)
          (bind _returnvalue (`|SpawnActorFromClass` "/Game/RoboValley/Blueprints/Platform/BP_Platform.BP_Platform_C" (`self.Spawn Transform_3`) "Undefined" "OverrideRootScale" null null))
          (bind _returnvalue_2 (`|SpawnActorFromClass` "/Game/RoboValley/Blueprints/Platform/BP_BreakingPlatform.BP_BreakingPlatform_C" (`self.Spawn Transform_2`) "Undefined" "OverrideRootScale" null null))
          (`KismetSystemLibrary.Delay` 2.0)
          (bind _returnvalue_3 (`|SpawnActorFromClass` "/Game/RoboValley/Blueprints/BP_WoodSpike.BP_WoodSpike_C" (`KismetMathLibrary.Conv_VectorToTransform` (`SceneComponent.K2_GetComponentLocation` (`self.Spawnpoint`))) "Undefined" "OverrideRootScale" null null))
          (bind _returnvalue_4 (`|SpawnActorFromClass` "/Game/RoboValley/Blueprints/BP_WoodSpike.BP_WoodSpike_C" (`KismetMathLibrary.Conv_VectorToTransform` (`SceneComponent.K2_GetComponentLocation` (`self.Spawnpoint2`))) "Undefined" "OverrideRootScale" null null))
          (bind _returnvalue_5 (`|SpawnActorFromClass` "/Game/RoboValley/Blueprints/BP_WoodSpike.BP_WoodSpike_C" (`KismetMathLibrary.Conv_VectorToTransform` (`SceneComponent.K2_GetComponentLocation` (`self.Spawnpoint3`))) "Undefined" "OverrideRootScale" null null))
          (bind _returnvalue_6 (`|SpawnActorFromClass` "/Game/RoboValley/Blueprints/BP_WoodSpike.BP_WoodSpike_C" (`KismetMathLibrary.Conv_VectorToTransform` (`SceneComponent.K2_GetComponentLocation` (`self.Spawnpoint4`))) "Undefined" "OverrideRootScale" null null))
          (`KismetSystemLibrary.Delay` 20.0)
          (`self.SetWarningScreenVisible`)
          (`self.SetWarningScreenHidden`)
          (`KismetSystemLibrary.Delay` 1.0)
          (set `self.IsSpikeSpawned?` false)
          (set `self.IsEventPlayed?` false)
          (`self.K2_DestroyActor` _returnvalue_3)
          (`self.K2_DestroyActor` _returnvalue_4)
          (`self.K2_DestroyActor` _returnvalue)
          (`self.K2_DestroyActor` _returnvalue_2)
          (`self.K2_DestroyActor` _returnvalue_5)
          (`self.K2_DestroyActor` _returnvalue_6)))
      (elif (not (`self.IsSpikeSpawned?`))
        (goto _label_4 :!via `Reset`)))))

(fn `UserConstructionScript`)