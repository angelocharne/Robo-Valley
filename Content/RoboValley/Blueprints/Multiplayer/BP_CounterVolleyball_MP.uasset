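; Scoring actor for two-player RoboValley volleyball, with a left and a right counter trigger that detect the ball.
; On BeginPlay it caches the main HUD and sets both players' win messages on the game mode.
; A ball overlap increments the opposite side's HUD score, teleports the ball to the scoring player's spawn point and zeroes its velocity.
; Each point also resets both robots' MinY/MaxY limits to fixed per-side values.
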(event `self.ReceiveBeginPlay`
  (bind _asmain_hud (cast `/Game/RoboValley/Blueprints/UI/MainHud` (`PlayerController.GetHUD` (`GameplayStatics.GetPlayerController` 0))))
  (set `self.MainHud REF` _asmain_hud)
  (bind _asrobo_valley_game_mode (cast `/Game/RoboValley/Game/RoboValleyGameMode` (`GameplayStatics.GetGameMode`)))
  (set `/Game/RoboValley/Game/RoboValleyGameMode.WinP2` "Player 2 Win!" _asrobo_valley_game_mode)
  (set `/Game/RoboValley/Game/RoboValleyGameMode.WinP1` "Player 1 Win!" _asrobo_valley_game_mode))

(event `self.RightCounter.OnComponentBeginOverlap`
  (params (OverlappedComponent :type "PrimitiveComponent Object Reference") (OtherActor :type "Actor Object Reference") (OtherComp :type "PrimitiveComponent Object Reference") (OtherBodyIndex :type Integer) (bFromSweep :type Boolean) (SweepResult :type "HitResult Structure (by ref)"))
  (bind _robop2_ref (`self.RoboP2 REF`))
  (bind _robop1_ref (`self.RoboP1 REF`))
  (bind _asbp_ball (cast `/Game/RoboValley/Blueprints/BP_Ball` OtherActor))
  (`/Engine/EditorBlueprintResources/StandardMacros.IncrementInt` (`/Game/RoboValley/Blueprints/UI/WBS_PointCounter.ScoreL` (`/Game/RoboValley/Blueprints/UI/MainHud.WBS PointCounter REF` (`self.MainHud REF`)))
    (:`  `
      (`self.K2_SetActorLocation` _asbp_ball (`SceneComponent.K2_GetComponentLocation` (`/Game/RoboValley/Blueprints/Character/BP_RoboP1.Ballspawnpoint` (`self.RoboP1 REF`))) false true)
      (`PrimitiveComponent.SetPhysicsLinearVelocity` (`/Game/RoboValley/Blueprints/BP_Ball.Sphere` _asbp_ball) (0.0 0.0 0.0) false "None")
      (set `/Game/RoboValley/Blueprints/Character/BP_RoboP1.MinY` -800.0 _robop1_ref)
      (set `/Game/RoboValley/Blueprints/Character/BP_RoboP1.MaxY` -1200.0 _robop1_ref)
      (set `/Game/RoboValley/Blueprints/Character/BP_RoboP2.MinY` 800.0 _robop2_ref)
      (set `/Game/RoboValley/Blueprints/Character/BP_RoboP2.MaxY` 1200.0 _robop2_ref))))

(event `self.LeftCounter.OnComponentBeginOverlap`
  (params (OverlappedComponent :type "PrimitiveComponent Object Reference") (OtherActor :type "Actor Object Reference") (OtherComp :type "PrimitiveComponent Object Reference") (OtherBodyIndex :type Integer) (bFromSweep :type Boolean) (SweepResult :type "HitResult Structure (by ref)"))
  (bind _robop2_ref (`self.RoboP2 REF`))
  (bind _robop1_ref (`self.RoboP1 REF`))
  (bind _asbp_ball (cast `/Game/RoboValley/Blueprints/BP_Ball` OtherActor))
  (`/Engine/EditorBlueprintResources/StandardMacros.IncrementInt` (`/Game/RoboValley/Blueprints/UI/WBS_PointCounter.ScoreR` (`/Game/RoboValley/Blueprints/UI/MainHud.WBS PointCounter REF` (`self.MainHud REF`)))
    (:`  `
      (`self.K2_SetActorLocation` _asbp_ball (`SceneComponent.K2_GetComponentLocation` (`/Game/RoboValley/Blueprints/Character/BP_RoboP2.Ballspawnpoint` (`self.RoboP2 REF`))) false true)
      (`PrimitiveComponent.SetPhysicsLinearVelocity` (`/Game/RoboValley/Blueprints/BP_Ball.Sphere` _asbp_ball) (0.0 0.0 0.0) false "None")
      (set `/Game/RoboValley/Blueprints/Character/BP_RoboP2.MinY` 800.0 _robop2_ref)
      (set `/Game/RoboValley/Blueprints/Character/BP_RoboP2.MaxY` 1200.0 _robop2_ref)
      (set `/Game/RoboValley/Blueprints/Character/BP_RoboP1.MinY` -800.0 _robop1_ref)
      (set `/Game/RoboValley/Blueprints/Character/BP_RoboP1.MaxY` -1200.0 _robop1_ref))))

(fn `UserConstructionScript`)