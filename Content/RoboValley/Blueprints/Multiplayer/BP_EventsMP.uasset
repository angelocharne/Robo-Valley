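; BP_EventsMP is a multiplayer RoboValley actor running timed gameplay events: breaking ground, spikes, and player shrink or grow.
; Counter values gate spikes and size changes; BreakGround follows the ground's disappearance state, and nothing wired here calls these events.
; A shared IsEventPlayed flag and resettable DoOnces prevent overlap, while Delay chains flash materials, restore scale and destroy spawned platforms and spikes.
; A box overlap teleports BP_RoboChar to its PlayerStart.
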(event `self.ReceiveTick`
  (params (DeltaSeconds :type "Float (single-precision)")))

(event `self.ReceiveBeginPlay`
  (bind _asmain_hud (cast `/Game/RoboValley/Blueprints/UI/MainHud` (`PlayerController.GetHUD` (`GameplayStatics.GetPlayerController` 0))))
  (set `self.MainHud REF` _asmain_hud)
  (bind _asrobo_valley_game_mode (cast `/Game/RoboValley/Game/RoboValleyGameMode` (`GameplayStatics.GetGameMode`)))
  (set `self.Gamemode REF` _asrobo_valley_game_mode))

(event `BreakGround`
  (bind _ground (`self.Ground`))
  (if (not (`self.IsEventPlayed?`))
    (`/Game/RoboValley/Blueprints/Multiplayer/BP_GroundMP.Ground Disapear` _ground)
    (if (`/Game/RoboValley/Blueprints/Multiplayer/BP_GroundMP.IsGroundDisapear?` _ground)
      (`/Engine/EditorBlueprintResources/StandardMacros.DoOnce` false :!label _label
        (:`Completed`
          (set `self.IsEventPlayed?` true)
          (set `self.IsPlatformSpawned?` true)
          (bind _returnvalue (`|SpawnActorFromClass` "/Game/RoboValley/Blueprints/Platform/BP_MovingPlatform2D.BP_MovingPlatform2D_C" (`self.Spawn Transform_1`) "Undefined" "OverrideRootScale" null null))
          (bind _returnvalue_2 (`|SpawnActorFromClass` "/Game/RoboValley/Blueprints/Platform/BP_BreakingPlatform.BP_BreakingPlatform_C" (`self.Spawn Transform`) "Undefined" "OverrideRootScale" null null))
          (bind _returnvalue_3 (`|SpawnActorFromClass` "/Game/RoboValley/Blueprints/Platform/BP_MovingPlatform2D.BP_MovingPlatform2D_C" (`self.Spawn Transform_0`) "Undefined" "OverrideRootScale" null null))
          (`SceneComponent.K2_SetWorldLocation` (`/Game/RoboValley/Blueprints/Platform/BP_MovingPlatform2D.Endpoint` _returnvalue_3) (1200.0 800.0 900.0) false false)
          (`KismetSystemLibrary.Delay` 23.0)
          (set `self.IsPlatformSpawned?` false)
          (set `self.IsEventPlayed?` false)
          (`self.K2_DestroyActor` _returnvalue)
          (`self.K2_DestroyActor` _returnvalue_2)
          (`self.K2_DestroyActor` _returnvalue_3)))
      (elif (not (`self.IsPlatformSpawned?`))
        (goto _label :!via `Reset`)))))

(event `self.Box.OnComponentBeginOverlap`
  (params (OverlappedComponent :type "PrimitiveComponent Object Reference") (OtherActor :type "Actor Object Reference") (OtherComp :type "PrimitiveComponent Object Reference") (OtherBodyIndex :type Integer) (bFromSweep :type Boolean) (SweepResult :type "HitResult Structure (by ref)"))
  (bind _asbp_robo_char (cast `/Game/RoboValley/Blueprints/Character/BP_RoboChar` OtherActor))
  (`self.K2_SetActorLocation` _asbp_robo_char (`SceneComponent.K2_GetComponentLocation` (`Actor.RootComponent` (`/Game/RoboValley/Blueprints/Character/BP_RoboChar.PlayerStart` _asbp_robo_char))) false true))

(event `Shrink`
  (bind _player_ref (`self.Player REF`))
  (bind _counter_ref (`self.Counter REF`))
  (bind _mesh (`Character.Mesh` _player_ref))
  ;[1 1 1] Shrink the player
  (if (not (`self.IsEventPlayed?`))
    (if (or (== (`/Game/RoboValley/Blueprints/Multiplayer/BP_CounterVolleyball_MP.Counter Left` _counter_ref) 6) (== (`/Game/RoboValley/Blueprints/Multiplayer/BP_CounterVolleyball_MP.Counter Right` _counter_ref) 6))
      (`/Engine/EditorBlueprintResources/StandardMacros.DoOnce` false :!label _label_2
        (:`Completed`
          (set `self.IsShrinked?` true)
          (set `self.IsEventPlayed?` true)
          (`PrimitiveComponent.SetMaterial` _mesh 0 "/Game/RoboValley/Material/Red.Red")
          (`KismetSystemLibrary.Delay` 0.3)
          (`PrimitiveComponent.SetMaterial` _mesh 0 null)
          (`KismetSystemLibrary.Delay` 0.3)
          (`PrimitiveComponent.SetMaterial` _mesh 0 "/Game/RoboValley/Material/Red.Red")
          (`KismetSystemLibrary.Delay` 0.2)
          (`PrimitiveComponent.SetMaterial` _mesh 0 null)
          (`KismetSystemLibrary.Delay` 0.2)
          (`PrimitiveComponent.SetMaterial` _mesh 0 "/Game/RoboValley/Material/Red.Red")
          (`KismetSystemLibrary.Delay` 0.2)
          (`PrimitiveComponent.SetMaterial` _mesh 0 null)
          (`KismetSystemLibrary.Delay` 0.2)
          (`PrimitiveComponent.SetMaterial` _mesh 0 "/Game/RoboValley/Material/Red.Red")
          (`self.SetActorScale3D` _player_ref (0.3 0.3 0.3))
          (`PrimitiveComponent.SetMaterial` _mesh 0 null)
          (`KismetSystemLibrary.Delay` 10.0)
          (`PrimitiveComponent.SetMaterial` _mesh 0 "/Game/RoboValley/Material/Green.Green")
          (`KismetSystemLibrary.Delay` 0.3)
          (`PrimitiveComponent.SetMaterial` _mesh 0 null)
          (`KismetSystemLibrary.Delay` 0.3)
          (`PrimitiveComponent.SetMaterial` _mesh 0 "/Game/RoboValley/Material/Green.Green")
          (`KismetSystemLibrary.Delay` 0.2)
          (`PrimitiveComponent.SetMaterial` _mesh 0 null)
          (`KismetSystemLibrary.Delay` 0.2)
          (`PrimitiveComponent.SetMaterial` _mesh 0 "/Game/RoboValley/Material/Green.Green")
          (`KismetSystemLibrary.Delay` 0.2)
          (`PrimitiveComponent.SetMaterial` _mesh 0 null)
          (`KismetSystemLibrary.Delay` 0.2)
          (`PrimitiveComponent.SetMaterial` _mesh 0 "/Game/RoboValley/Material/Green.Green")
          (`KismetSystemLibrary.Delay` 0.2)
          (set `self.IsShrinked?` false)
          (set `self.IsEventPlayed?` false)
          (`PrimitiveComponent.SetMaterial` _mesh 0 null)
          (`self.SetActorScale3D` (`self.Player REF`) (1.0 1.0 1.0))))
      (elif (not (`self.IsShrinked?`))
        (goto _label_2 :!via `Reset`)))))

(event `Grow`
  (bind _player_ref (`self.Player REF`))
  (bind _counter_ref (`self.Counter REF`))
  (bind _mesh (`Character.Mesh` _player_ref))
  (bind _mesh_2 (`Character.Mesh` _player_ref))
  ;[1 1 1] Event Grow Up Player
  (if (not (`self.IsEventPlayed?`))
    (if (or (== (`/Game/RoboValley/Blueprints/Multiplayer/BP_CounterVolleyball_MP.Counter Left` _counter_ref) 7) (== (`/Game/RoboValley/Blueprints/Multiplayer/BP_CounterVolleyball_MP.Counter Right` _counter_ref) 7))
      (`/Engine/EditorBlueprintResources/StandardMacros.DoOnce` false :!label _label_3
        (:`Completed`
          (set `self.IsGrowed` true)
          (set `self.IsEventPlayed?` true)
          (`PrimitiveComponent.SetMaterial` _mesh 0 "/Game/RoboValley/Material/Green.Green")
          (`KismetSystemLibrary.Delay` 0.3)
          (`PrimitiveComponent.SetMaterial` _mesh 0 null)
          (`KismetSystemLibrary.Delay` 0.3)
          (`PrimitiveComponent.SetMaterial` _mesh 0 "/Game/RoboValley/Material/Green.Green")
          (`KismetSystemLibrary.Delay` 0.2)
          (`PrimitiveComponent.SetMaterial` _mesh 0 null)
          (`KismetSystemLibrary.Delay` 0.2)
          (`PrimitiveComponent.SetMaterial` _mesh 0 "/Game/RoboValley/Material/Green.Green")
          (`KismetSystemLibrary.Delay` 0.2)
          (`PrimitiveComponent.SetMaterial` _mesh 0 null)
          (`KismetSystemLibrary.Delay` 0.2)
          (`PrimitiveComponent.SetMaterial` _mesh 0 "/Game/RoboValley/Material/Green.Green")
          (`KismetSystemLibrary.Delay` 0.2)
          (`PrimitiveComponent.SetMaterial` _mesh 0 null)
          (`self.SetActorScale3D` _player_ref (2.5 2.5 2.5))
          (`KismetSystemLibrary.Delay` 10.0)
          (`PrimitiveComponent.SetMaterial` _mesh_2 0 "/Game/RoboValley/Material/Red.Red")
          (`KismetSystemLibrary.Delay` 0.3)
          (`PrimitiveComponent.SetMaterial` _mesh_2 0 null)
          (`KismetSystemLibrary.Delay` 0.3)
          (`PrimitiveComponent.SetMaterial` _mesh_2 0 "/Game/RoboValley/Material/Red.Red")
          (`KismetSystemLibrary.Delay` 0.2)
          (`PrimitiveComponent.SetMaterial` _mesh_2 0 null)
          (`KismetSystemLibrary.Delay` 0.2)
          (`PrimitiveComponent.SetMaterial` _mesh_2 0 "/Game/RoboValley/Material/Red.Red")
          (`KismetSystemLibrary.Delay` 0.2)
          (`PrimitiveComponent.SetMaterial` _mesh_2 0 null)
          (`KismetSystemLibrary.Delay` 0.2)
          (`PrimitiveComponent.SetMaterial` _mesh_2 0 "/Game/RoboValley/Material/Red.Red")
          (`KismetSystemLibrary.Delay` 0.2)
          (`PrimitiveComponent.SetMaterial` _mesh_2 0 null)
          (set `self.IsGrowed` false)
          (set `self.IsEventPlayed?` false)
          (`self.SetActorScale3D` _player_ref (1.0 1.0 1.0))))
      (elif (not (`self.IsGrowed`))
        (goto _label_3 :!via `Reset`)))))

(event `Spikes`
  (bind _counter_ref (`self.Counter REF`))
  (if (not (`self.IsEventPlayed?`))
    (if (or (== (`/Game/RoboValley/Blueprints/Multiplayer/BP_CounterVolleyball_MP.Counter Left` _counter_ref) 2) (== (`/Game/RoboValley/Blueprints/Multiplayer/BP_CounterVolleyball_MP.Counter Right` _counter_ref) 2))
      (`/Engine/EditorBlueprintResources/StandardMacros.DoOnce` false :!label _label_4
        (:`Completed`
          (set `self.IsEventPlayed?` true)
          (set `self.IsSpikeSpawned?` true)
          (bind _returnvalue (`|SpawnActorFromClass` "/Game/RoboValley/Blueprints/Platform/BP_Platform.BP_Platform_C" (`self.Spawn Transform_3`) "Undefined" "OverrideRootScale" null null))
          (bind _returnvalue_2 (`|SpawnActorFromClass` "/Game/RoboValley/Blueprints/Platform/BP_BreakingPlatform.BP_BreakingPlatform_C" (`self.Spawn Transform_2`) "Undefined" "OverrideRootScale" null null))
          (`KismetSystemLibrary.Delay` 2.0)
          (bind _returnvalue_3 (`|SpawnActorFromClass` "/Game/RoboValley/Blueprints/BP_WoodSpike.BP_WoodSpike_C" (`KismetMathLibrary.Conv_VectorToTransform` (`SceneComponent.K2_GetComponentLocation` (`self.Spawnpoint`))) "Undefined" "OverrideRootScale" null null))
          (bind _returnvalue_4 (`|SpawnActorFromClass` "/Game/RoboValley/Blueprints/BP_WoodSpike.BP_WoodSpike_C" (`KismetMathLibrary.Conv_VectorToTransform` (`SceneComponent.K2_GetComponentLocation` (`self.Spawnpoint2`))) "Undefined" "OverrideRootScale" null null))
          (bind _returnvalue_5 (`|SpawnActorFromClass` "/Game/RoboValley/Blueprints/BP_WoodSpike.BP_WoodSpike_C" (`KismetMathLibrary.Conv_VectorToTransform` (`SceneComponent.K2_GetComponentLocation` (`self.Spawnpoint3`))) "Undefined" "OverrideRootScale" null null))
          (bind _returnvalue_6 (`|SpawnActorFromClass` "/Game/RoboValley/Blueprints/BP_WoodSpike.BP_WoodSpike_C" (`KismetMathLibrary.Conv_VectorToTransform` (`SceneComponent.K2_GetComponentLocation` (`self.Spawnpoint4`))) "Undefined" "OverrideRootScale" null null))
          (`KismetSystemLibrary.Delay` 15.0)
          (set `self.IsSpikeSpawned?` false)
          (set `self.IsEventPlayed?` false)
          (`self.K2_DestroyActor` _returnvalue_3)
          (`self.K2_DestroyActor` _returnvalue_4)
          (`self.K2_DestroyActor` _returnvalue)
          (`self.K2_DestroyActor` _returnvalue_2)
          (`self.K2_DestroyActor` _returnvalue_5)
          (`self.K2_DestroyActor` _returnvalue_6)))
      (elif (not (`self.IsSpikeSpawned?`))
        (goto _label_4 :!via `Reset`)))))

(fn `UserConstructionScript`)