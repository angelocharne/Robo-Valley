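; Moving one-way platform in RoboValley multiplayer that shuttles between two points and breaks under BP_RoboP2.
; A looping FlipFlop timeline lerps the Cube back and forth, while CollisionTrigger blocks Pawns only when the robot is above it.
; A hit starts a Tick-based frame counter, reset on leaving PhasedTrigger, that triggers BreakingPlatform to swap meshes, drop collision and restore.
; BetterBreaking, a physics-based variant, is not called within this Blueprint.
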(event `self.ReceiveBeginPlay`
  ;[1 1 1] Set The Collision on Begin Play off
  (`PrimitiveComponent.SetCollisionResponseToChannel` (`self.Cube`) "ECC_Pawn" "ECR_Ignore")
  (`self.From Start to End`)
  (set `self.Start Location` (`self.K2_GetActorLocation`))
  (`self.StartTimer`))

(event `self.Collision Trigger.OnComponentBeginOverlap`
  (params (OverlappedComponent :type "PrimitiveComponent Object Reference") (OtherActor :type "Actor Object Reference") (OtherComp :type "PrimitiveComponent Object Reference") (OtherBodyIndex :type Integer) (bFromSweep :type Boolean) (SweepResult :type "HitResult Structure (by ref)"))
  ;[1 1 1] If on begin overlap the box collision, enable Platform collision
  (bind _asbp_robo_p2 (cast `/Game/RoboValley/Blueprints/Character/BP_RoboP2` OtherActor))
  (if (> (.z (`SceneComponent.K2_GetComponentLocation` (`Character.Mesh` _asbp_robo_p2))) (.z (`SceneComponent.K2_GetComponentLocation` (`self.Cube`))))
    (`PrimitiveComponent.SetCollisionResponseToChannel` (`self.Cube`) "ECC_Pawn" "ECR_Block")))

(event `self.Collision Trigger.OnComponentEndOverlap`
  (params (OverlappedComponent :type "PrimitiveComponent Object Reference") (OtherActor :type "Actor Object Reference") (OtherComp :type "PrimitiveComponent Object Reference") (OtherBodyIndex :type Integer))
  ;[1 1 1] If on end overlap the box collision, disable Platform Collision
  (cast `/Game/RoboValley/Blueprints/Character/BP_RoboP2` OtherActor)
  (`PrimitiveComponent.SetCollisionResponseToChannel` (`self.Cube`) "ECC_Pawn" "ECR_Ignore"))

(event `From Start to End`
  (`KismetSystemLibrary.Delay` (`self.Delay Timer`))
  (`/Engine/EditorBlueprintResources/StandardMacros.FlipFlop`
    (:`A`
      (bind (_direction _alpha) (`Timeline|Alpha Lerp` :!via `PlayFromStart` :!label _label)
        (:`Update`
          (`SceneComponent.K2_SetWorldLocation` (`self.Cube`) (`KismetMathLibrary.VLerp` (`SceneComponent.K2_GetComponentLocation` (`self.Startpoint`)) (`SceneComponent.K2_GetComponentLocation` (`self.Endpoint`)) _alpha) false false))
        (:`Finished`
          (`self.From Start to End`))))
    (:`B`
      (goto _label :!via `ReverseFromEnd`))))

(event `self.ReceiveTick`
  (params (DeltaSeconds :type "Float (single-precision)"))
  (if (`self.IsPlayerOnPlatform?`)
    (`self.StartTimer`)
    (if (== (`self.Timer`) 175)
      (`self.BreakingPlatform`))))

(event `self.Cube.OnComponentHit`
  (params (HitComponent :type "PrimitiveComponent Object Reference") (OtherActor :type "Actor Object Reference") (OtherComp :type "PrimitiveComponent Object Reference") (NormalImpulse :type "Vector Structure") (Hit :type "HitResult Structure (by ref)"))
  (cast `/Game/RoboValley/Blueprints/Character/BP_RoboP2` OtherActor)
  (set `self.IsPlayerOnPlatform?` true))

(event `self.Phased Trigger.OnComponentEndOverlap`
  (params (OverlappedComponent :type "PrimitiveComponent Object Reference") (OtherActor :type "Actor Object Reference") (OtherComp :type "PrimitiveComponent Object Reference") (OtherBodyIndex :type Integer))
  (cast `/Game/RoboValley/Blueprints/Character/BP_RoboP2` OtherActor)
  (set `self.IsPlayerOnPlatform?` false)
  (set `self.Timer` 0))

(event `BreakingPlatform`
  (bind _cube (`self.Cube`))
  (bind _staticmesh1 (`self.StaticMesh1`))
  (`SceneComponent.SetHiddenInGame` (`self.Cube`) true false)
  (`SceneComponent.SetHiddenInGame` (`self.StaticMesh`) true false)
  (`SceneComponent.SetHiddenInGame` _staticmesh1 false false)
  (`SceneComponent.SetHiddenInGame` (`self.StaticMesh2`) false false)
  (`KismetSystemLibrary.Delay` 0.45)
  (`PrimitiveComponent.SetMaterial` _staticmesh1 0 "/Game/RoboValley/Material/Red.Red")
  (`PrimitiveComponent.SetMaterial` (`self.StaticMesh2`) 0 "/Game/RoboValley/Material/Red.Red")
  (`PrimitiveComponent.SetCollisionEnabled` (`self.Cube`) "NoCollision")
  (`SceneComponent.SetHiddenInGame` (`self.StaticMesh1`) true false)
  (`SceneComponent.SetHiddenInGame` (`self.StaticMesh2`) true false)
  (`KismetSystemLibrary.Delay` 0.8)
  (`SceneComponent.SetHiddenInGame` _cube false false)
  (`SceneComponent.SetHiddenInGame` (`self.StaticMesh`) false false)
  (`PrimitiveComponent.SetCollisionEnabled` _cube "QueryAndPhysics")
  (`PrimitiveComponent.SetMaterial` (`self.StaticMesh1`) 0 null)
  (`PrimitiveComponent.SetMaterial` (`self.StaticMesh2`) 0 null))

(event `BetterBreaking`
  (set `self.IsPlayerOnPlatform?` true)
  (`KismetSystemLibrary.Delay` 2.0)
  (`SceneComponent.SetHiddenInGame` (`self.Cube`) true false)
  (`SceneComponent.SetHiddenInGame` (`self.StaticMesh`) true false)
  (`SceneComponent.SetHiddenInGame` (`self.StaticMesh1`) false false)
  (`SceneComponent.SetHiddenInGame` (`self.StaticMesh2`) false false)
  (`KismetSystemLibrary.Delay` 0.25)
  (`PrimitiveComponent.SetSimulatePhysics` (`self.Cube`) true)
  (`KismetSystemLibrary.Delay` 1.5)
  (`SceneComponent.SetHiddenInGame` (`self.StaticMesh1`) true false)
  (`SceneComponent.SetHiddenInGame` (`self.StaticMesh2`) true false)
  (`KismetSystemLibrary.Delay` 0.5)
  (`SceneComponent.SetHiddenInGame` (`self.Cube`) false false)
  (`SceneComponent.SetHiddenInGame` (`self.StaticMesh`) false false)
  (`PrimitiveComponent.SetSimulatePhysics` (`self.Cube`) false)
  (`SceneComponent.K2_SetWorldLocation` (`self.Cube`) (`self.Start Location`) false false)
  (set `self.IsPlayerOnPlatform?` false))

(fn `StartTimer`
  (`/Engine/EditorBlueprintResources/StandardMacros.IncrementInt` (`self.Timer`)))

(fn `UserConstructionScript`)