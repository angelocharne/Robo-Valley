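; BP_Platform1 is a one-way side-scroller platform in RoboValley's multiplayer content, letting BP_RoboP2 pass through from below and stand on top.
; Its cube ignores Pawns by default, blocking them when BP_RoboP2 overlaps CollisionTrigger from above and ignoring again on exit.
; PhasedTrigger toggles player 0's input and a gate for SideScrollerCharacters, with the gate's exit disabling collision to drop through, though no gate entry is shown.
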(event `self.ReceiveBeginPlay`
  ;[1 1 1] Set The Collision on Begin Play off
  (`PrimitiveComponent.SetCollisionResponseToChannel` (`self.Cube`) "ECC_Pawn" "ECR_Ignore"))

(event `self.Collision Trigger.OnComponentBeginOverlap`
  (params (OverlappedComponent :type "PrimitiveComponent Object Reference") (OtherActor :type "Actor Object Reference") (OtherComp :type "PrimitiveComponent Object Reference") (OtherBodyIndex :type Integer) (bFromSweep :type Boolean) (SweepResult :type "HitResult Structure (by ref)"))
  ;[1 1 1] If on begin overlap the box collision, enable Platform collision
  (bind _asbp_robo_p2 (cast `/Game/RoboValley/Blueprints/Character/BP_RoboP2` OtherActor))
  (if (> (.z (`SceneComponent.K2_GetComponentLocation` (`Character.Mesh` _asbp_robo_p2))) (.z (`SceneComponent.K2_GetComponentLocation` (`self.Cube`))))
    (`PrimitiveComponent.SetCollisionResponseToChannel` (`self.Cube`) "ECC_Pawn" "ECR_Block")))

(event `self.Collision Trigger.OnComponentEndOverlap`
  (params (OverlappedComponent :type "PrimitiveComponent Object Reference") (OtherActor :type "Actor Object Reference") (OtherComp :type "PrimitiveComponent Object Reference") (OtherBodyIndex :type Integer))
  ;[1 1 1] If on end overlap the box collision, disable Platform Collision
  (cast `/Game/RoboValley/Blueprints/Character/BP_RoboP2` OtherActor)
  (`PrimitiveComponent.SetCollisionResponseToChannel` (`self.Cube`) "ECC_Pawn" "ECR_Ignore"))

(event `self.Phased Trigger.OnComponentBeginOverlap`
  (params (OverlappedComponent :type "PrimitiveComponent Object Reference") (OtherActor :type "Actor Object Reference") (OtherComp :type "PrimitiveComponent Object Reference") (OtherBodyIndex :type Integer) (bFromSweep :type Boolean) (SweepResult :type "HitResult Structure (by ref)"))
  ;[1 1 1] Phased out of the Platform
  (cast `/Game/RoboValley/Blueprints/SideScrollerExample/SideScrollerCharacter` OtherActor)
  (`self.EnableInput` (`GameplayStatics.GetPlayerController` 0))
  (`/Engine/EditorBlueprintResources/StandardMacros.Gate` true :!via `Open` :!label _label
    (:`Exit`
      (`PrimitiveComponent.SetCollisionResponseToChannel` (`self.Cube`) "ECC_Pawn" "ECR_Ignore"))))

(event `self.Phased Trigger.OnComponentEndOverlap`
  (params (OverlappedComponent :type "PrimitiveComponent Object Reference") (OtherActor :type "Actor Object Reference") (OtherComp :type "PrimitiveComponent Object Reference") (OtherBodyIndex :type Integer))
  ;[1 1 1] Phased out of the Platform
  (cast `/Game/RoboValley/Blueprints/SideScrollerExample/SideScrollerCharacter` OtherActor)
  (`self.DisableInput` (`GameplayStatics.GetPlayerController` 0))
  (set `self.Counter` 0)
  (goto _label :!via `Close`))

(fn `UserConstructionScript`)