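; BP_GroundMP is a multiplayer ground piece that temporarily disappears when either the left or right counter reaches three.
; GroundDisapear runs a delayed sequence: the main cube swaps to two sub-cubes, which turn red, then all three hide and lose collision.
; After a long delay, the main cube reappears and collision and materials are restored.
; A DoOnce blocks retriggering, resetting on calls where neither counter is three and the sequence is inactive.
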(event `Ground Disapear`
  (bind _counter_ref (`self.Counter REF`))
  (bind _cube (`self.Cube`))
  (if (or (== (`/Game/RoboValley/Blueprints/Multiplayer/BP_CounterVolleyball_MP.Counter Left` _counter_ref) 3) (== (`/Game/RoboValley/Blueprints/Multiplayer/BP_CounterVolleyball_MP.Counter Right` _counter_ref) 3))
    (`/Engine/EditorBlueprintResources/StandardMacros.DoOnce` false :!label _label
      (:`Completed`
        (set `self.IsGroundDisapear?` true)
        (`KismetSystemLibrary.Delay` 1.0)
        (`SceneComponent.SetHiddenInGame` _cube true false)
        (`PrimitiveComponent.SetCollisionEnabled` _cube "NoCollision")
        (`SceneComponent.SetHiddenInGame` (`self.Cube2`) false false)
        (`SceneComponent.SetHiddenInGame` (`self.Cube1`) false false)
        (`KismetSystemLibrary.Delay` 1.0)
        (`PrimitiveComponent.SetMaterial` (`self.Cube1`) 0 "/Game/RoboValley/Material/Red.Red")
        (`PrimitiveComponent.SetMaterial` (`self.Cube2`) 0 "/Game/RoboValley/Material/Red.Red")
        (`KismetSystemLibrary.Delay` 0.8)
        (`SceneComponent.SetHiddenInGame` (`self.Cube`) true false)
        (`SceneComponent.SetHiddenInGame` (`self.Cube1`) true false)
        (`SceneComponent.SetHiddenInGame` (`self.Cube2`) true false)
        (`PrimitiveComponent.SetCollisionEnabled` (`self.Cube`) "NoCollision")
        (`PrimitiveComponent.SetCollisionEnabled` (`self.Cube1`) "NoCollision")
        (`PrimitiveComponent.SetCollisionEnabled` (`self.Cube2`) "NoCollision")
        (`KismetSystemLibrary.Delay` 20.0)
        (set `self.IsGroundDisapear?` false)
        (`SceneComponent.SetHiddenInGame` (`self.Cube`) false false)
        (`PrimitiveComponent.SetCollisionEnabled` (`self.Cube`) "QueryAndPhysics")
        (`PrimitiveComponent.SetCollisionEnabled` (`self.Cube1`) "QueryAndPhysics")
        (`PrimitiveComponent.SetCollisionEnabled` (`self.Cube2`) "QueryAndPhysics")
        (`PrimitiveComponent.SetMaterial` (`self.Cube`) 0 "/Game/RoboValley/Material/NewMaterial.NewMaterial")
        (`PrimitiveComponent.SetMaterial` (`self.Cube1`) 0 "/Game/RoboValley/Material/NewMaterial.NewMaterial")
        (`PrimitiveComponent.SetMaterial` (`self.Cube2`) 0 "/Game/RoboValley/Material/NewMaterial.NewMaterial")))
    (elif (not (`self.IsGroundDisapear?`))
      (goto _label :!via `Reset`))))

(fn `UserConstructionScript`)