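; BP_Ground is a platform piece that temporarily disappears after a screen warning.
; GroundDisapear runs a delayed sequence, swapping the main Cube for two substitute cubes, turning them red, then hiding them and disabling collision.
; After a longer wait it signals the warning again through BPEvent, clears IsGroundDisapear, then restores the main Cube and all collision.
; The substitute cubes stay hidden and are never reset from red.
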(event `Ground Disapear`
  (bind _cube1 (`self.Cube1`))
  (bind _bp_event (`self.BP_Event`))
  (bind _bp_event_2 (`self.BP_Event`))
  (bind _cube (`self.Cube`))
  (`/Game/RoboValley/Blueprints/BP_Events.SetWarningScreenVisible` _bp_event)
  (`/Game/RoboValley/Blueprints/BP_Events.SetWarningScreenHidden` _bp_event)
  (`KismetSystemLibrary.Delay` 3.0)
  (`SceneComponent.SetHiddenInGame` _cube true false)
  (`PrimitiveComponent.SetCollisionEnabled` _cube "NoCollision")
  (`SceneComponent.SetHiddenInGame` (`self.Cube2`) false false)
  (`SceneComponent.SetHiddenInGame` _cube1 false false)
  (`KismetSystemLibrary.Delay` 0.8)
  (`PrimitiveComponent.SetMaterial` _cube1 0 "/Game/RoboValley/Material/Red.Red")
  (`PrimitiveComponent.SetMaterial` (`self.Cube2`) 0 "/Game/RoboValley/Material/Red.Red")
  (`KismetSystemLibrary.Delay` 0.8)
  (`SceneComponent.SetHiddenInGame` _cube1 true false)
  (`SceneComponent.SetHiddenInGame` (`self.Cube2`) true false)
  (`PrimitiveComponent.SetCollisionEnabled` (`self.Cube1`) "NoCollision")
  (`PrimitiveComponent.SetCollisionEnabled` (`self.Cube2`) "NoCollision")
  (`KismetSystemLibrary.Delay` 20.0)
  (`/Game/RoboValley/Blueprints/BP_Events.SetWarningScreenVisible` _bp_event_2)
  (`/Game/RoboValley/Blueprints/BP_Events.SetWarningScreenHidden` _bp_event_2)
  (set `self.IsGroundDisapear?` false)
  (`KismetSystemLibrary.Delay` 1.0)
  (`SceneComponent.SetHiddenInGame` (`self.Cube`) false false)
  (`PrimitiveComponent.SetCollisionEnabled` (`self.Cube`) "QueryAndPhysics")
  (`PrimitiveComponent.SetCollisionEnabled` (`self.Cube2`) "QueryAndPhysics")
  (`PrimitiveComponent.SetCollisionEnabled` (`self.Cube1`) "QueryAndPhysics"))

(fn `UserConstructionScript`)