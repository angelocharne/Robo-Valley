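; Falling platform for RoboValley that the player can land on from above and that briefly vanishes after being touched.
; CollisionTrigger makes the Cube block pawns only when the player's mesh is higher than it, and ignore them again on exit, giving one-way collision.
; A BP_RoboChar overlapping Box starts delays that swap the material, hide the platform without collision, then restore it.
; Nothing moves the actor; its saved start location is unused.
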(event `self.ReceiveBeginPlay`
  ;[1 1 1] Set The Collision on Begin Play off
  (`PrimitiveComponent.SetCollisionResponseToChannel` (`self.Cube`) "ECC_Pawn" "ECR_Ignore")
  (set `self.Start Location` (`self.K2_GetActorLocation`)))

(event `self.Collision Trigger.OnComponentBeginOverlap`
  (params (OverlappedComponent :type "PrimitiveComponent Object Reference") (OtherActor :type "Actor Object Reference") (OtherComp :type "PrimitiveComponent Object Reference") (OtherBodyIndex :type Integer) (bFromSweep :type Boolean) (SweepResult :type "HitResult Structure (by ref)"))
  (bind _returnvalue (`GameplayStatics.GetPlayerCharacter` 0))
  ;[1 1 1] If on begin overlap the box collision, enable Platform collision
  (if (== OtherActor _returnvalue)
    (if (> (.z (`SceneComponent.K2_GetComponentLocation` (`Character.Mesh` _returnvalue))) (.z (`SceneComponent.K2_GetComponentLocation` (`self.Cube`))))
      (`PrimitiveComponent.SetCollisionResponseToChannel` (`self.Cube`) "ECC_Pawn" "ECR_Block"))))

(event `self.Collision Trigger.OnComponentEndOverlap`
  (params (OverlappedComponent :type "PrimitiveComponent Object Reference") (OtherActor :type "Actor Object Reference") (OtherComp :type "PrimitiveComponent Object Reference") (OtherBodyIndex :type Integer))
  ;[1 1 1] If on end overlap the box collision, disable Platform Collision
  (if (== OtherActor (`GameplayStatics.GetPlayerCharacter` 0))
    (`PrimitiveComponent.SetCollisionResponseToChannel` (`self.Cube`) "ECC_Pawn" "ECR_Ignore")))

(event `self.Box.OnComponentBeginOverlap`
  (params (OverlappedComponent :type "PrimitiveComponent Object Reference") (OtherActor :type "Actor Object Reference") (OtherComp :type "PrimitiveComponent Object Reference") (OtherBodyIndex :type Integer) (bFromSweep :type Boolean) (SweepResult :type "HitResult Structure (by ref)"))
  (bind _cube (`self.Cube`))
  (cast `/Game/RoboValley/Blueprints/Character/BP_RoboChar` OtherActor)
  (`KismetSystemLibrary.Delay` 0.2)
  (`KismetSystemLibrary.Delay` 2.0)
  (`PrimitiveComponent.SetMaterial` (`self.StaticMesh`) 0 "/Game/RoboValley/Material/NewMaterial1.NewMaterial1")
  (`KismetSystemLibrary.Delay` 1.0)
  (`SceneComponent.SetHiddenInGame` (`self.Cube`) true false)
  (`SceneComponent.SetHiddenInGame` (`self.StaticMesh`) true false)
  (`PrimitiveComponent.SetCollisionEnabled` (`self.Cube`) "NoCollision")
  (`KismetSystemLibrary.Delay` 0.3)
  (`SceneComponent.SetHiddenInGame` _cube false false)
  (`SceneComponent.SetHiddenInGame` (`self.StaticMesh`) false false)
  (`PrimitiveComponent.SetCollisionEnabled` _cube "QueryAndPhysics")
  (`PrimitiveComponent.SetMaterial` (`self.StaticMesh`) 0 null))

(fn `UserConstructionScript`)