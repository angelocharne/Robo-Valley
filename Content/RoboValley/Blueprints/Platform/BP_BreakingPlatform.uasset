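; Breakable one-way platform that gives way shortly after the player character hits it, then restores itself.
; The Cube ignores Pawns by default, and a trigger volume switches it to Block while the player is inside, provided they entered from above.
; A player hit swaps the intact meshes for two alternate meshes, then chained delays turn those red, hide them with Cube collision off, and bring the platform back.
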(event `self.ReceiveBeginPlay`
  ;[1 1 1] Set The Collision on Begin Play off
  (`PrimitiveComponent.SetCollisionResponseToChannel` (`self.Cube`) "ECC_Pawn" "ECR_Ignore")
  (set `self.Start Location` (`self.K2_GetActorLocation`)))

(event `self.Collision Trigger.OnComponentBeginOverlap`
  (params (OverlappedComponent :type "PrimitiveComponent Object Reference") (OtherActor :type "Actor Object Reference") (OtherComp :type "PrimitiveComponent Object Reference") (OtherBodyIndex :type Integer) (bFromSweep :type Boolean) (SweepResult :type "HitResult Structure (by ref)"))
  (bind _returnvalue (`GameplayStatics.GetPlayerCharacter` 0))
  ;[1 1 1] If on begin overlap the box collision, enable Platform collision
  (if (== OtherActor _returnvalue)
    (if (or (> (.z (`SceneComponent.K2_GetComponentLocation` (`Character.Mesh` _returnvalue))) (.z (`SceneComponent.K2_GetComponentLocation` (`self.Cube`)))) false)
      (`PrimitiveComponent.SetCollisionResponseToChannel` (`self.Cube`) "ECC_Pawn" "ECR_Block"))))

(event `self.Collision Trigger.OnComponentEndOverlap`
  (params (OverlappedComponent :type "PrimitiveComponent Object Reference") (OtherActor :type "Actor Object Reference") (OtherComp :type "PrimitiveComponent Object Reference") (OtherBodyIndex :type Integer))
  ;[1 1 1] If on end overlap the box collision, disable Platform Collision
  (if (== OtherActor (`GameplayStatics.GetPlayerCharacter` 0))
    (`PrimitiveComponent.SetCollisionResponseToChannel` (`self.Cube`) "ECC_Pawn" "ECR_Ignore")))

(event `self.Cube.OnComponentHit`
  (params (HitComponent :type "PrimitiveComponent Object Reference") (OtherActor :type "Actor Object Reference") (OtherComp :type "PrimitiveComponent Object Reference") (NormalImpulse :type "Vector Structure") (Hit :type "HitResult Structure (by ref)"))
  (bind _staticmesh1 (`self.StaticMesh1`))
  (bind _cube (`self.Cube`))
  (if (== (`GameplayStatics.GetPlayerCharacter` 0) OtherActor)
    (`SceneComponent.SetHiddenInGame` (`self.Cube`) true false)
    (`SceneComponent.SetHiddenInGame` (`self.StaticMesh`) true false)
    (`SceneComponent.SetHiddenInGame` _staticmesh1 false false)
    (`SceneComponent.SetHiddenInGame` (`self.StaticMesh2`) false false)
    (`KismetSystemLibrary.Delay` 0.8)
    (`PrimitiveComponent.SetMaterial` _staticmesh1 0 "/Game/RoboValley/Material/Red.Red")
    (`PrimitiveComponent.SetMaterial` (`self.StaticMesh2`) 0 "/Game/RoboValley/Material/Red.Red")
    (`KismetSystemLibrary.Delay` 0.5)
    (`PrimitiveComponent.SetCollisionEnabled` (`self.Cube`) "NoCollision")
    (`SceneComponent.SetHiddenInGame` (`self.StaticMesh1`) true false)
    (`SceneComponent.SetHiddenInGame` (`self.StaticMesh2`) true false)
    (`KismetSystemLibrary.Delay` 0.4)
    (`SceneComponent.SetHiddenInGame` _cube false false)
    (`SceneComponent.SetHiddenInGame` (`self.StaticMesh`) false false)
    (`PrimitiveComponent.SetCollisionEnabled` _cube "QueryAndPhysics")
    (`PrimitiveComponent.SetMaterial` (`self.StaticMesh1`) 0 null)
    (`PrimitiveComponent.SetMaterial` (`self.StaticMesh2`) 0 null)))

(fn `UserConstructionScript`)