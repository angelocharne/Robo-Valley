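; BP_CounterVolleyball_MP is a volleyball counter actor with left and right court triggers that react to BP_Ball.
; An overlap teleports the ball to the spawn point of PlayerREF (right field) or RoboP2REF (left field) and zeroes its velocity.
; It then sets the opposite side's counter to a random integer and prints it.
; The increment nodes for both counters are disconnected, so no real score accumulates.
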(event `self.RightCounter.OnComponentBeginOverlap`
  (params (OverlappedComponent :type "PrimitiveComponent Object Reference") (OtherActor :type "Actor Object Reference") (OtherComp :type "PrimitiveComponent Object Reference") (OtherBodyIndex :type Integer) (bFromSweep :type Boolean) (SweepResult :type "HitResult Structure (by ref)"))
  (bind _asbp_ball (cast `/Game/RoboValley/Blueprints/BP_Ball` OtherActor))
  (`KismetSystemLibrary.PrintString` "Hit the Right Field")
  (`self.K2_SetActorLocation` _asbp_ball (`SceneComponent.K2_GetComponentLocation` (`/Game/RoboValley/Blueprints/Character/BP_RoboChar.Ballspawnpoint` (`self.Player REF`))) false true)
  (`PrimitiveComponent.SetPhysicsLinearVelocity` (`/Game/RoboValley/Blueprints/BP_Ball.Sphere` _asbp_ball) (0.0 0.0 0.0) false "None")
  (set `self.Counter Left` (`KismetMathLibrary.RandomIntegerInRange` 0 8))
  (`KismetSystemLibrary.PrintString` (`KismetStringLibrary.Conv_IntToString` (`self.Counter Left`))))

(event `self.LeftCounter.OnComponentBeginOverlap`
  (params (OverlappedComponent :type "PrimitiveComponent Object Reference") (OtherActor :type "Actor Object Reference") (OtherComp :type "PrimitiveComponent Object Reference") (OtherBodyIndex :type Integer) (bFromSweep :type Boolean) (SweepResult :type "HitResult Structure (by ref)"))
  (bind _asbp_ball (cast `/Game/RoboValley/Blueprints/BP_Ball` OtherActor))
  (`KismetSystemLibrary.PrintString` "Hit the Left Field")
  (`self.K2_SetActorLocation` _asbp_ball (`SceneComponent.K2_GetComponentLocation` (`/Game/RoboValley/Blueprints/Character/BP_RoboP2.Ballspawnpoint` (`self.RoboP2 REF`))) false true)
  (`PrimitiveComponent.SetPhysicsLinearVelocity` (`/Game/RoboValley/Blueprints/BP_Ball.Sphere` _asbp_ball) (0.0 0.0 0.0) false "None")
  (set `self.Counter Right` (`KismetMathLibrary.RandomIntegerInRange` 0 8))
  (`KismetSystemLibrary.PrintString` (`KismetStringLibrary.Conv_IntToString` (`self.Counter Right`))))

(fn `UserConstructionScript`)