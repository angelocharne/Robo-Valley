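; BP_Jumping_AI is an AI controller that runs the BT_AI_Jumping behavior tree using the BB_AI_Jumping blackboard.
; On BeginPlay and every Tick it finds all BP_AI_TargetPoint actors and takes the first one.
; It writes a random reachable point in a small radius around that actor to the MoveLocation key, so the destination is re-rolled each frame.
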(event `self.ReceiveBeginPlay`
  (bind _blackboardcomponent (`self.UseBlackboard` "/Game/RoboValley/Blueprints/AI/BB_AI_Jumping.BB_AI_Jumping"))
  (set `self.CurrentBlackboard` _blackboardcomponent)
  (bind _outactors (`GameplayStatics.GetAllActorsOfClass` "/Game/RoboValley/Blueprints/AI/BP_AI_TargetPoint.BP_AI_TargetPoint_C"))
  (`BlackboardComponent.SetValueAsVector` (`self.CurrentBlackboard`) "MoveLocation" (`NavigationSystemV1.K2_GetRandomReachablePointInRadius` (`self.K2_GetActorLocation` (`|GetArrayItem` _outactors)) 25.0 null null))
  (`self.RunBehaviorTree` "/Game/RoboValley/Blueprints/AI/BT_AI_Jumping.BT_AI_Jumping"))

(event `self.ReceiveTick`
  (params (DeltaSeconds :type "Float (single-precision)"))
  (bind _outactors (`GameplayStatics.GetAllActorsOfClass` "/Game/RoboValley/Blueprints/AI/BP_AI_TargetPoint.BP_AI_TargetPoint_C"))
  (`BlackboardComponent.SetValueAsVector` (`self.CurrentBlackboard`) "MoveLocation" (`NavigationSystemV1.K2_GetRandomReachablePointInRadius` (`self.K2_GetActorLocation` (`|GetArrayItem` _outactors)) 25.0 null null)))

(fn `UserConstructionScript`)