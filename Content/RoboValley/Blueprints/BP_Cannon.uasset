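; BP_Cannon is a RoboValley cannon that moves back and forth and fires balls when it spots the side-scroller character.
; A timeline lerps the Cylinder between Startpunkt and Endpunkt, with a self-calling FlipFlop event alternating play and reverse.
; PawnSensing sightings start a delay, after which a BP_Ball spawns at the Ballspawner transform.
; A look-at rotation toward the player exists but is never executed.
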(event `self.ReceiveBeginPlay`
  ;[1 1 1] Comment
  (`KismetSystemLibrary.Delay` 0.5)
  (`self.Von Start zu Ende`))

(event `self.PawnSensing.OnSeePawn`
  (params (Pawn :type "Pawn Object Reference"))
  ;[1 1 1] Comment
  (bind _asside_scroller_character (cast `/Game/RoboValley/Blueprints/SideScrollerExample/SideScrollerCharacter` Pawn))
  (`|ExecutionSequence`
    (:`then_1`
      (`KismetSystemLibrary.Delay` 4.0)
      (`|SpawnActorFromClass` "/Game/RoboValley/Blueprints/BP_Ball.BP_Ball_C" (`SceneComponent.K2_GetComponentToWorld` (`self.Ballspawner`)) "Undefined" "OverrideRootScale" null null))))

(event `Von Start zu Ende`
  ;[1 1 1] Comment
  (`/Engine/EditorBlueprintResources/StandardMacros.FlipFlop`
    (:`A`
      (bind (_direction _newtrack_0) (`Timeline|Timeline_0` :!via `PlayFromStart` :!label _label)
        (:`Update`
          (`SceneComponent.K2_SetWorldLocation` (`self.Cylinder`) (`KismetMathLibrary.VLerp` (`SceneComponent.K2_GetComponentLocation` (`self.Startpunkt`)) (`SceneComponent.K2_GetComponentLocation` (`self.Endpunkt`)) _newtrack_0) false false))
        (:`Finished`
          (`self.Von Start zu Ende`))))
    (:`B`
      (goto _label :!via `ReverseFromEnd`))))

(fn `UserConstructionScript`)