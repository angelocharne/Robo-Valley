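; BP_WoodSpike is a moving spike hazard that sends BP_RoboChar back to its stored PlayerStart on contact.
; From BeginPlay, a timeline lerps the static mesh between Startpoint and Endpoint, with a FlipFlop alternating play and reverse each time it finishes for an endless back-and-forth.
; A Box overlap casts to BP_RoboChar and teleports it to that PlayerStart's location.
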(event `self.ReceiveBeginPlay`
  (`self.From Start to End`))

(event `self.Box.OnComponentBeginOverlap`
  (params (OverlappedComponent :type "PrimitiveComponent Object Reference") (OtherActor :type "Actor Object Reference") (OtherComp :type "PrimitiveComponent Object Reference") (OtherBodyIndex :type Integer) (bFromSweep :type Boolean) (SweepResult :type "HitResult Structure (by ref)"))
  (bind _asbp_robo_char (cast `/Game/RoboValley/Blueprints/Character/BP_RoboChar` OtherActor))
  (`self.K2_SetActorLocation` _asbp_robo_char (`SceneComponent.K2_GetComponentLocation` (`Actor.RootComponent` (`/Game/RoboValley/Blueprints/Character/BP_RoboChar.PlayerStart` _asbp_robo_char))) false true))

(event `From Start to End`
  (`/Engine/EditorBlueprintResources/StandardMacros.FlipFlop`
    (:`A`
      (bind (_direction _alpha) (`Timeline|Timeline_0` :!via `PlayFromStart` :!label _label)
        (:`Update`
          (`SceneComponent.K2_SetWorldLocation` (`self.StaticMesh`) (`KismetMathLibrary.VLerp` (`SceneComponent.K2_GetComponentLocation` (`self.Startpoint`)) (`SceneComponent.K2_GetComponentLocation` (`self.Endpoint`)) _alpha) false false))
        (:`Finished`
          (`self.From Start to End`))))
    (:`B`
      (goto _label :!via `ReverseFromEnd`))))

(fn `UserConstructionScript`)