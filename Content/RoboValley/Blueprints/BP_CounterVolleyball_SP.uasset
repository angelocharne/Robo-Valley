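; Single-player volleyball score counter that detects when the ball lands in the left or right field and awards the point to the opposite side.
; Overlaps on two counter components increment the score on the HUD's point counter widget, cached at BeginPlay.
; The ball then teleports to the player's or robot AI's spawn point with zeroed velocity.
; Right-field hits also reset the AI's MinY/MaxY range.
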(event `self.ReceiveBeginPlay`
  (bind _asmain_hud (cast `/Game/RoboValley/Blueprints/UI/MainHud` (`PlayerController.GetHUD` (`GameplayStatics.GetPlayerController` 0))))
  (set `self.Hud REF` _asmain_hud))

(event `self.RightCounter.OnComponentBeginOverlap`
  (params (OverlappedComponent :type "PrimitiveComponent Object Reference") (OtherActor :type "Actor Object Reference") (OtherComp :type "PrimitiveComponent Object Reference") (OtherBodyIndex :type Integer) (bFromSweep :type Boolean) (SweepResult :type "HitResult Structure (by ref)"))
  (bind _roboai_ref (`self.RoboAI REF`))
  (bind _asbp_ball (cast `/Game/RoboValley/Blueprints/BP_Ball` OtherActor))
  (`KismetSystemLibrary.PrintString` "Hit the Right Field")
  (`/Engine/EditorBlueprintResources/StandardMacros.IncrementInt` (`/Game/RoboValley/Blueprints/UI/WBS_PointCounter.ScoreL` (`/Game/RoboValley/Blueprints/UI/MainHud.WBS PointCounter REF` (`self.Hud REF`)))
    (:`  `
      (`self.K2_SetActorLocation` _asbp_ball (`SceneComponent.K2_GetComponentLocation` (`/Game/RoboValley/Blueprints/Character/BP_RoboChar.Ballspawnpoint` (`self.Player REF`))) false true)
      (`PrimitiveComponent.SetPhysicsLinearVelocity` (`/Game/RoboValley/Blueprints/BP_Ball.Sphere` _asbp_ball) (0.0 0.0 0.0) false "None")
      (set `/Game/RoboValley/Blueprints/AI/BP_RoboAI.MinY` 1000.0 _roboai_ref)
      (set `/Game/RoboValley/Blueprints/AI/BP_RoboAI.MaxY` 1400.0 _roboai_ref))))

(event `self.LeftCounter.OnComponentBeginOverlap`
  (params (OverlappedComponent :type "PrimitiveComponent Object Reference") (OtherActor :type "Actor Object Reference") (OtherComp :type "PrimitiveComponent Object Reference") (OtherBodyIndex :type Integer) (bFromSweep :type Boolean) (SweepResult :type "HitResult Structure (by ref)"))
  (bind _asbp_ball (cast `/Game/RoboValley/Blueprints/BP_Ball` OtherActor))
  (`KismetSystemLibrary.PrintString` "Hit the Left Field")
  (`/Engine/EditorBlueprintResources/StandardMacros.IncrementInt` (`/Game/RoboValley/Blueprints/UI/WBS_PointCounter.ScoreR` (`/Game/RoboValley/Blueprints/UI/MainHud.WBS PointCounter REF` (`self.Hud REF`)))
    (:`  `
      (`self.K2_SetActorLocation` _asbp_ball (`SceneComponent.K2_GetComponentLocation` (`/Game/RoboValley/Blueprints/AI/BP_RoboAI.Ballspawnpoint` (`self.RoboAI REF`))) false true)
      (`PrimitiveComponent.SetPhysicsLinearVelocity` (`/Game/RoboValley/Blueprints/BP_Ball.Sphere` _asbp_ball) (0.0 0.0 0.0) false "None"))))

(fn `UserConstructionScript`)