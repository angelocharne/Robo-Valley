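; BP_GrowDown is a RoboValley item that temporarily shrinks the robot character when BP_RoboP2 touches it.
; Its static mesh's begin overlap fires once, scaling RoboCharREF down and restoring full scale after a ten-second delay.
; When BP_RoboP2 leaves the mesh, the item hides and waits the same length of time before destroying itself.
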(event `self.StaticMesh.OnComponentBeginOverlap`
  (params (OverlappedComponent :type "PrimitiveComponent Object Reference") (OtherActor :type "Actor Object Reference") (OtherComp :type "PrimitiveComponent Object Reference") (OtherBodyIndex :type Integer) (bFromSweep :type Boolean) (SweepResult :type "HitResult Structure (by ref)"))
  (bind _robochar_ref (`self.RoboChar REF`))
  (cast `/Game/RoboValley/Blueprints/Character/BP_RoboP2` OtherActor)
  (`/Engine/EditorBlueprintResources/StandardMacros.DoOnce` false
    (:`Completed`
      (`self.SetActorScale3D` _robochar_ref (0.3 0.3 0.3))
      (`KismetSystemLibrary.Delay` 10.0)
      (`self.SetActorScale3D` _robochar_ref (1.0 1.0 1.0)))))

(event `self.StaticMesh.OnComponentEndOverlap`
  (params (OverlappedComponent :type "PrimitiveComponent Object Reference") (OtherActor :type "Actor Object Reference") (OtherComp :type "PrimitiveComponent Object Reference") (OtherBodyIndex :type Integer))
  (cast `/Game/RoboValley/Blueprints/Character/BP_RoboP2` OtherActor)
  (`self.SetActorHiddenInGame` true)
  (`KismetSystemLibrary.Delay` 10.0)
  (`self.K2_DestroyActor`))

(fn `UserConstructionScript`)